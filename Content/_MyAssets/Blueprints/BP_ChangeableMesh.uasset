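; Changeable mesh actor that cycles its static mesh, material and color through configured lists.
; BeginPlay applies the active ModelData mesh and material as a dynamic instance tinted through the "color" parameter.
; Three events step their index with wraparound: mesh swaps apply that model's first material, material swaps use the active model's list.
; Both swaps set materials untinted; color changes create a new dynamic instance from the current material.
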(event Custom|ChangeMeshInOrder
  ;[1 1 1] change mesh in order
  (if (< (Variables|Default|GetactiveModelIndex) (Utilities|Array|Length (Variables|Default|GetModelData)))
    (if (== (+ (Variables|Default|GetactiveModelIndex) 1) (Utilities|Array|Length (Variables|Default|GetModelData)))
      (Variables|Default|SetactiveModelIndex 0)
      (else
        (Variables|Default|SetactiveModelIndex (+ (Variables|Default|GetactiveModelIndex) 1))))
    (else
      (Variables|Default|SetactiveModelIndex 0)))
  (Components|StaticMesh|SetStaticMesh (Variables|Default|GetStaticMesh1) (.StaticMesh (Utilities|Struct|BreakModelData (Utilities|Array|Get(acopy) (Variables|Default|GetModelData) (Variables|Default|GetactiveModelIndex)))))
  (Rendering|Material|SetMaterial (Variables|Default|GetStaticMesh1) 0 (Utilities|Array|Get(acopy) (.Materials (Utilities|Struct|BreakModelData (Utilities|Array|Get(acopy) (Variables|Default|GetModelData) (Variables|Default|GetactiveModelIndex)))))))

(event Custom|changeColorInOrder
  ;[1 1 1] change color in order
  (if (< (Variables|Default|GetactiveColorIndex) (Utilities|Array|Length (Variables|Default|GetColors)))
    (if (== (+ (Variables|Default|GetactiveColorIndex) 1) (Utilities|Array|Length (Variables|Default|GetColors)))
      (Variables|Default|SetactiveColorIndex 0)
      (else
        (Variables|Default|SetactiveColorIndex (+ (Variables|Default|GetactiveColorIndex) 1))))
    (else
      (Variables|Default|SetactiveColorIndex 0)))
  (bind _returnvalue (Rendering|Material|CreateDynamicMaterialInstance (Variables|Default|GetStaticMesh1) 0 (Rendering|Material|GetMaterial (Variables|Default|GetStaticMesh1) 0) "None" :!class /Script/Engine.PrimitiveComponent))
  (bind _output_get (Variables|Default|SetcoloredMaterial _returnvalue))
  (Rendering|Material|SetVectorParameterValue _output_get "color" (Utilities|Array|Get(acopy) (Variables|Default|GetColors) (Variables|Default|GetactiveColorIndex)) :!class /Script/Engine.MaterialInstanceDynamic)
  (Rendering|Material|SetMaterial (Variables|Default|GetStaticMesh1) 0 (Variables|Default|GetcoloredMaterial)))

(event Custom|ChangeMaterialInOrder
  ;[1 1 1] change material in order
  (if (< (Variables|Default|GetactiveMaterialIndex) (Utilities|Array|Length (.Materials (Utilities|Struct|BreakModelData (Utilities|Array|Get(acopy) (Variables|Default|GetModelData) (Variables|Default|GetactiveModelIndex))))))
    (if (== (+ (Variables|Default|GetactiveMaterialIndex) 1) (Utilities|Array|Length (.Materials (Utilities|Struct|BreakModelData (Utilities|Array|Get(acopy) (Variables|Default|GetModelData) (Variables|Default|GetactiveModelIndex))))))
      (Variables|Default|SetactiveMaterialIndex 0)
      (else
        (Variables|Default|SetactiveMaterialIndex (+ (Variables|Default|GetactiveMaterialIndex) 1))))
    (else
      (Variables|Default|SetactiveMaterialIndex 0)))
  (Rendering|Material|SetMaterial (Variables|Default|GetStaticMesh1) 0 (Utilities|Array|Get(acopy) (.Materials (Utilities|Struct|BreakModelData (Utilities|Array|Get(acopy) (Variables|Default|GetModelData) (Variables|Default|GetactiveModelIndex)))) (Variables|Default|GetactiveMaterialIndex))))

(event EventBeginPlay
  (bind _modeldata (Variables|Default|GetModelData))
  (bind _activemodelindex (Variables|Default|GetactiveModelIndex))
  (bind _output (Utilities|Array|Get(acopy) _modeldata _activemodelindex))
  (bind (_staticmesh _materials) (Utilities|Struct|BreakModelData _output))
  (Components|StaticMesh|SetStaticMesh (Variables|Default|GetStaticMesh1) _staticmesh)
  (bind _returnvalue (Rendering|Material|CreateDynamicMaterialInstance (Variables|Default|GetStaticMesh1) 0 (Utilities|Array|Get(acopy) _materials (Variables|Default|GetactiveMaterialIndex)) "None" :!class /Script/Engine.PrimitiveComponent))
  (bind _output_get (Variables|Default|SetcoloredMaterial _returnvalue))
  (Rendering|Material|SetVectorParameterValue _output_get "color" (Utilities|Array|Get(acopy) (Variables|Default|GetColors) (Variables|Default|GetactiveColorIndex)) :!class /Script/Engine.MaterialInstanceDynamic)
  (Rendering|Material|SetMaterial (Variables|Default|GetStaticMesh1) 0 (Variables|Default|GetcoloredMaterial)))

(fn ConstructionScript)